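; BP_DrawingBoard_Foliage is a drawing board child that records brush strokes into render targets that fade over time, apparently for foliage.
; Before simulation it renders the saved target into the output target, where brushes draw.
; Afterwards a dynamic M_TurbulenceFade material copies the output back to the saved target, fading it by delta time over FadeTime.
; Fade time and saved target come from a foliage data asset, with sleep time set slightly longer.
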(event EventBeginPlay
  (|CallParentFunction))

(event EventPostSimulate
  (bind _simulatematerial (Variables|Default|GetSimulateMaterial))
  (|CallParentFunction)
  (Rendering|Material|SetTextureParameterValue _simulatematerial "CopyFrom" (Variables|Default|GetOutput%20RT))
  (Rendering|Material|SetScalarParameterValue _simulatematerial "FadeStrength" (/ (Utilities|Time|GetWorldDeltaSeconds) (Variables|Default|GetFadeTime)) :!class /Script/Engine.MaterialInstanceDynamic)
  (Rendering|DrawMaterialtoRenderTarget (Variables|Default|GetSaveRT) _simulatematerial))

(event EventPreSimulate
  (|CallParentFunction)
  (CallFunction|RenderPrevioustoCurrent (Variables|Default|GetSaveRT) (Variables|Default|GetOutput%20RT))
  (Variables|Default|SetRTBrushDrawOn (Variables|Default|GetOutput%20RT)))

(fn ConstructionScript
  (|CallParentFunction))

(fn InitializewithDataAsset
  (params (Data :type BP%20Drawing%20Board%20Data%20Object%20Reference))
  (|CallParentFunction Data)
  (bind _returnvalue (Rendering|Material|CreateDynamicMaterialInstance "/InteractiveWorld/Materials/DrawingBoardMaterials/FoliageSimulateMaterials/M_TurbulenceFade.M_TurbulenceFade" "None" "None" :!class /Script/Engine.KismetMaterialLibrary))
  (Variables|Default|SetSimulateMaterial _returnvalue)
  (bind _asbp_drawing_board_data_foliage (Utilities|Casting|CastToBP_DrawingBoardData_Foliage (Variables|Default|GetDataAsset)))
  (bind _output_get (Variables|Default|SetFadeTime (Variables|/InteractiveWorld/Blueprints/DataAssets/BP_DrawingBoardData_Foliage.BP_DrawingBoardData_Foliage_C|GetFadeTime _asbp_drawing_board_data_foliage)))
  (Variables|Default|SetSleepTime (+ _output_get 0.5))
  (bind _output_get_2 (Variables|Default|SetSaveRT (Variables|/InteractiveWorld/Blueprints/DataAssets/BP_DrawingBoardData_Foliage.BP_DrawingBoardData_Foliage_C|GetSaveRT _asbp_drawing_board_data_foliage)))
  (Rendering|ClearRenderTarget2D _output_get_2))