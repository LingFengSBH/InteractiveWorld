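; World affector scene component that gives its owning actor shape, turbulent and fluid brushes from a single placed component.
; On BeginPlay it creates the three brush components at runtime, attaches them to itself and sets the shape brush's type.
; Its world scale, times 100, sizes them once: shape bounds in 3D, turbulent and fluid size from XY, and their interact distance from half Z.
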(event EventBeginPlay
  (bind _returnvalue (Transformation|GetWorldScale))
  (bind _returnvalue_2 (* _returnvalue 1e+02))
  (bind _returnvalue_3 (Math|Conversions|ToVector2D(Vector) _returnvalue_2))
  (bind _z (Math|Vector|BreakVector _returnvalue_2))
  (bind _returnvalue_4 (/ _z 2.0))
  (Utilities|FlowControl|Sequence
    (:then_0
      (bind _returnvalue_5 (Game|AddComponentbyClass (Components|GetOwner) "/InteractiveWorld/Blueprints/Brushes/BP_Brush_Shape.BP_Brush_Shape_C" true))
      (bind _output_get (Variables|Default|SetBP_Brush_Shape _returnvalue_5))
      (Transformation|AttachComponentToComponent _output_get self "None" "KeepRelative" "KeepRelative" "KeepRelative" false)
      (Variables|/InteractiveWorld/Blueprints/Brushes/BP_Brush_Shape.BP_Brush_Shape_C|SetShape _output_get "NewEnumerator0"))
    (:then_1
      (bind _returnvalue_6 (Game|AddComponentbyClass (Components|GetOwner) "/InteractiveWorld/Blueprints/Brushes/BP_Brush_Turbulent.BP_Brush_Turbulent_C" true))
      (bind _output_get_2 (Variables|Default|SetBP_Brush_Turbulent _returnvalue_6))
      (Transformation|AttachComponentToComponent _output_get_2 self "None" "KeepRelative" "KeepRelative" "KeepRelative" false))
    (:then_2
      (bind _returnvalue_7 (Game|AddComponentbyClass (Components|GetOwner) "/InteractiveWorld/Blueprints/Brushes/BP_Brush_Fluid.BP_Brush_Fluid_C" true))
      (bind _output_get_3 (Variables|Default|SetBP_Brush_Fluid _returnvalue_7))
      (Transformation|AttachComponentToComponent _output_get_3 self "None" "KeepRelative" "KeepRelative" "KeepRelative" false))
    (:then_3
      (Default|ResetBounds (Variables|Default|GetBP_Brush_Shape) _returnvalue_2)
      (Variables|/Script/InteractiveWorld.InteractBrush|SetSize (Variables|Default|GetBP_Brush_Fluid) _returnvalue_3)
      (Variables|/Script/InteractiveWorld.InteractBrush|SetSize (Variables|Default|GetBP_Brush_Turbulent) _returnvalue_3)
      (Variables|/InteractiveWorld/Blueprints/Brushes/Master/BP_MasterInteractBrush.BP_MasterInteractBrush_C|SetInteractDistance (Variables|Default|GetBP_Brush_Fluid) _returnvalue_4)
      (Variables|/InteractiveWorld/Blueprints/Brushes/Master/BP_MasterInteractBrush.BP_MasterInteractBrush_C|SetInteractDistance (Variables|Default|GetBP_Brush_Turbulent) _returnvalue_4))))