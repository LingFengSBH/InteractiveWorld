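; Fluid variant of the drawing board Blueprint, driving a fluid simulation through the PNSFluid component, which it activates on BeginPlay.
; Data asset initialization supplies the velocity input render target.
; Each board state update clears OutputRT to black and sets it as the brush's draw target.
; Before simulating, it passes the current-to-previous matrix offset to User.Offset so the simulation can account for board movement.
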(event EventBeginPlay
  (|CallParentFunction)
  (Components|Activation|SetActive (Variables|Default|GetP_NS_Fluid) true true))

(event Collision|EventActorBeginOverlap
  (params (OtherActor :type Actor%20Object%20Reference)))

(event EventUpdateDrawingBoardState
  (bind _output_rt (Variables|Default|GetOutput%20RT))
  (|CallParentFunction)
  (Rendering|ClearRenderTarget2D _output_rt)
  (Variables|Default|SetRTBrushDrawOn _output_rt))

(event EventEndPlay
  (params (EndPlayReason :type EEndPlayReason%20Enum :default "Destroyed")))

(event EventPreSimulate
  (bind _offset (CallFunction|CurrenttoPreviousMatrix))
  (|CallParentFunction)
  (Class|NiagaraComponent|SetVariableVec2 (Variables|Default|GetP_NS_Fluid) "User.Offset" (Math|Vector2D|MakeVector2D (.x _offset) (.y _offset))))

(fn ConstructionScript
  (|CallParentFunction))

(fn InitializewithDataAsset
  (params (Data :type BP%20Drawing%20Board%20Data%20Object%20Reference))
  (|CallParentFunction Data)
  (bind _asbp_drawing_board_data_fluid (Utilities|Casting|CastToBP_DrawingBoardData_Fluid Data))
  (Variables|Default|SetVelocity%20Input%20RT (Variables|/InteractiveWorld/Blueprints/DataAssets/BP_DrawingBoardData_Fluid.BP_DrawingBoardData_Fluid_C|GetVelocityInputRT _asbp_drawing_board_data_fluid)))