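; BP_MasterInteractBrush is a base brush for surface interaction, with an empty DrawonRT event that suggests child brushes handle render target drawing.
; UpdateDrawInfo saves the previous height and returns whether interaction applies, using one of three modes: always, landscape line trace or fixed-height plane.
; The trace hits WorldStatic objects vertically within InteractDistance, recording height and impact point.
; Plane mode uses absolute vertical distance to InteractPlane.
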(event EventBeginPlay)

(event EventTick
  (params (DeltaSeconds :type Float%20%28single-precision%29)))

(event EventDrawonRT
  (params (DrawingBoard :type World%20Drawing%20Board%20Object%20Reference) (CanvasDrawOn :type Canvas%20Object%20Reference) (CanvasSize :type Vector%202D%20Structure) (InterpolateRate :type Float%20%28single-precision%29) (DrawTimes :type Integer)))

(fn UpdateDrawInfo
  (Variables|TraceInfo|SetPreviousHeight (Variables|TraceInfo|GetHeight))
  (switch Utilities|FlowControl|Switch|SwitchonE_InteractMode (Variables|InteracMode|GetInteractMode)
    (:NewEnumerator0
      _)
    (:NewEnumerator1
      (|LineTrace
        (:Succeed
          _)
        (:Fail
          (return false))))
    (:NewEnumerator2
      (|HeightPlane
        (:Succeed
          _)
        (:Fail
          (return false)))))
  (return true))