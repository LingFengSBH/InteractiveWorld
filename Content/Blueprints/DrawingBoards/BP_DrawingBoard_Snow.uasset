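; Snow drawing board that simulates a deformable snow surface in render targets, configured by a BP_DrawingBoardData_Snow asset.
; Each step, an edge material combines the frame's brush render target with the previous state, using noise-driven bank parameters.
; High quality adds a shadow and detail-noise pass, then copies state back; low quality uses a simpler material and ping-pongs targets.
; Surface color, thickness and quality flag go to a material parameter collection.
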(event EventBeginPlay
  (|CallParentFunction))

(event EventPreSimulate
  (bind _output_rt (Variables|Default|GetOutput%20RT))
  (|CallParentFunction)
  (Rendering|ClearRenderTarget2D _output_rt)
  (Variables|Default|SetRTBrushDrawOn _output_rt))

(event EventUpdateDrawingBoardState
  (CallFunction|UpdateSimulateLocation true (Math|Float|SelectFloat 1.0 2.0 (Variables|Default|GetLowQuality))))

(event EventPostSimulate
  (bind _edgemat (Variables|Default|GetEdgeMat))
  (bind _shadow (Variables|Default|GetShadow))
  (|CallParentFunction)
  (Rendering|Material|SetTextureParameterValue _edgemat "Previous" (Variables|Default|GetPrevious))
  (Rendering|Material|SetTextureParameterValue _edgemat "CurrentFrame" (Variables|Default|GetRTBrushDrawOn))
  (CallFunction|SetCurrenttoPreviousMaterialParam _edgemat)
  (Rendering|DrawMaterialtoRenderTarget (Variables|Default|GetCurrent) _edgemat)
  (if (Variables|Default|GetLowQuality)
    (bind (_canvas _size _context) (Rendering|BeginDrawCanvastoRenderTarget (Variables|Default|GetOutput%20RT)))
    (Canvas|DrawTexture :self _canvas :RenderTexture (Variables|Default|GetCurrent) :ScreenSize _size :CoordinateSize "(X=1.000000,Y=1.000000)" :BlendMode "BLEND_Opaque" :PivotPoint "(X=0.500000,Y=0.500000)")
    (Rendering|EndDrawCanvastoRenderTarget _context)
    (CallFunction|SwitchRTs)
    (else
      (Rendering|Material|SetTextureParameterValue _shadow "Texture" (Variables|Default|GetCurrent))
      (Rendering|DrawMaterialtoRenderTarget (Variables|Default|GetOutput%20RT) _shadow)
      (Rendering|DrawMaterialtoRenderTarget (Variables|Default|GetPrevious) "/InteractiveWorld/Materials/DrawingBoardMaterials/SnowSimulateMaterials/SimulateMaterials/M_SnowCopy.M_SnowCopy"))))

(fn ConstructionScript
  (|CallParentFunction)
  (bind _asbp_drawing_board_data_snow (Utilities|Casting|CastToBP_DrawingBoardData_Snow (Variables|Default|GetDataAsset)))
  (Rendering|Material|SetVectorParameterValue (Variables|Default|GetBoardMPC) (Utilities|Name|MakeLiteralName "SnowSurfaceColor") (Variables|/InteractiveWorld/Blueprints/DataAssets/BP_DrawingBoardData_Snow.BP_DrawingBoardData_Snow_C|GetSnowSubSurfaceColor _asbp_drawing_board_data_snow) :!class /Script/Engine.KismetMaterialLibrary))

(fn InitializewithDataAsset
  (params (Data :type BP%20Drawing%20Board%20Data%20Object%20Reference))
  (bind _canvasworldsize (Variables|Default|GetCanvasWorldSize))
  (bind _boardmpc (Variables|Default|GetBoardMPC))
  (|CallParentFunction Data)
  (bind _asbp_drawing_board_data_snow (Utilities|Casting|CastToBP_DrawingBoardData_Snow (Variables|Default|GetDataAsset)))
  (LocalVariables|SetSnowData _asbp_drawing_board_data_snow)
  (Variables|Default|SetInteractHeight (Variables|/InteractiveWorld/Blueprints/DataAssets/BP_DrawingBoardData_Snow.BP_DrawingBoardData_Snow_C|GetSnowThickness (LocalVariables|GetSnowData)))
  (Variables|Default|SetLowQuality (Variables|/InteractiveWorld/Blueprints/DataAssets/BP_DrawingBoardData_Snow.BP_DrawingBoardData_Snow_C|GetUseLowQuality (LocalVariables|GetSnowData)))
  (Utilities|FlowControl|Sequence
    (:then_0
      (Variables|Default|SetSleepTime (Math|Float|SelectFloat 0.0 (+ (Variables|/InteractiveWorld/Blueprints/DataAssets/BP_DrawingBoardData_Snow.BP_DrawingBoardData_Snow_C|GetFreshSnowFallTime (LocalVariables|GetSnowData)) 0.1) (Variables|Default|GetLowQuality))))
    (:then_1
      (bind _returnvalue (Rendering|Material|CreateDynamicMaterialInstance (select (Variables|Default|GetLowQuality) "/InteractiveWorld/Materials/DrawingBoardMaterials/SnowSimulateMaterials/SimulateMaterials/M_RT_DrawEdge_Simple.M_RT_DrawEdge_Simple" "/InteractiveWorld/Materials/DrawingBoardMaterials/SnowSimulateMaterials/SimulateMaterials/M_RT_DrawEdge.M_RT_DrawEdge") "None" "None" :!class /Script/Engine.KismetMaterialLibrary))
      (bind _output_get (Variables|Default|SetEdgeMat _returnvalue))
      (Rendering|Material|SetTextureParameterValue _output_get "Noise" (Variables|/InteractiveWorld/Blueprints/DataAssets/BP_DrawingBoardData_Snow.BP_DrawingBoardData_Snow_C|GetBankBaseNoise (LocalVariables|GetSnowData)))
      (Rendering|Material|SetVectorParameterValue _output_get "SizeRange" (Math|Color|MakeColor (.X (Math|Vector2D|BreakVector2D (Variables|/InteractiveWorld/Blueprints/DataAssets/BP_DrawingBoardData_Snow.BP_DrawingBoardData_Snow_C|GetBankBaseNoiseSize (LocalVariables|GetSnowData)))) (.Y (Math|Vector2D|BreakVector2D (Variables|/InteractiveWorld/Blueprints/DataAssets/BP_DrawingBoardData_Snow.BP_DrawingBoardData_Snow_C|GetBankBaseNoiseSize (LocalVariables|GetSnowData)))) (.X (Math|Vector2D|BreakVector2D (Variables|/InteractiveWorld/Blueprints/DataAssets/BP_DrawingBoardData_Snow.BP_DrawingBoardData_Snow_C|GetBankBaseNoiseRange (LocalVariables|GetSnowData)))) (.Y (Math|Vector2D|BreakVector2D (Variables|/InteractiveWorld/Blueprints/DataAssets/BP_DrawingBoardData_Snow.BP_DrawingBoardData_Snow_C|GetBankBaseNoiseRange (LocalVariables|GetSnowData))))) :!class /Script/Engine.MaterialInstanceDynamic)
      (Rendering|Material|SetScalarParameterValue _output_get "DistanceU" (/ (Variables|/InteractiveWorld/Blueprints/DataAssets/BP_DrawingBoardData_Snow.BP_DrawingBoardData_Snow_C|GetBankWidth (LocalVariables|GetSnowData)) (.x _canvasworldsize)) :!class /Script/Engine.MaterialInstanceDynamic)
      (Rendering|Material|SetScalarParameterValue _output_get "DistanceV" (/ (Variables|/InteractiveWorld/Blueprints/DataAssets/BP_DrawingBoardData_Snow.BP_DrawingBoardData_Snow_C|GetBankWidth (LocalVariables|GetSnowData)) (.y _canvasworldsize)) :!class /Script/Engine.MaterialInstanceDynamic)
      (Rendering|Material|SetScalarParameterValue _output_get "BankIntencity" (Variables|/InteractiveWorld/Blueprints/DataAssets/BP_DrawingBoardData_Snow.BP_DrawingBoardData_Snow_C|GetBankIntensity (LocalVariables|GetSnowData)) :!class /Script/Engine.MaterialInstanceDynamic)
      (Rendering|Material|SetTextureParameterValue _output_get "Texture" (Variables|Default|GetOutput%20RT)))
    (:then_2
      (if (not (Variables|Default|GetLowQuality))
        (bind _returnvalue_2 (Rendering|Material|CreateDynamicMaterialInstance "/InteractiveWorld/Materials/DrawingBoardMaterials/SnowSimulateMaterials/SimulateMaterials/M_RT_Shadow.M_RT_Shadow" "None" "None" :!class /Script/Engine.KismetMaterialLibrary))
        (bind _output_get_2 (Variables|Default|SetShadow _returnvalue_2))
        (Rendering|Material|SetTextureParameterValue _output_get_2 "Noise" (Variables|/InteractiveWorld/Blueprints/DataAssets/BP_DrawingBoardData_Snow.BP_DrawingBoardData_Snow_C|GetBankDetailNoise (LocalVariables|GetSnowData)))
        (Rendering|Material|SetVectorParameterValue _output_get_2 "SizeRange" (Math|Color|MakeColor (.X (Math|Vector2D|BreakVector2D (Variables|/InteractiveWorld/Blueprints/DataAssets/BP_DrawingBoardData_Snow.BP_DrawingBoardData_Snow_C|GetBankDetailNoiseSize (LocalVariables|GetSnowData)))) (.Y (Math|Vector2D|BreakVector2D (Variables|/InteractiveWorld/Blueprints/DataAssets/BP_DrawingBoardData_Snow.BP_DrawingBoardData_Snow_C|GetBankDetailNoiseSize (LocalVariables|GetSnowData)))) (* (Variables|/InteractiveWorld/Blueprints/DataAssets/BP_DrawingBoardData_Snow.BP_DrawingBoardData_Snow_C|GetBankDetailNoiseIntensity (LocalVariables|GetSnowData)) -1.0) (Variables|/InteractiveWorld/Blueprints/DataAssets/BP_DrawingBoardData_Snow.BP_DrawingBoardData_Snow_C|GetBankDetailNoiseIntensity (LocalVariables|GetSnowData))) :!class /Script/Engine.MaterialInstanceDynamic)
        (CallFunction|SetMaterialCanvasParameters _output_get_2)
        (Rendering|Material|SetScalarParameterValue _output_get_2 "SnowThickness" (Variables|/InteractiveWorld/Blueprints/DataAssets/BP_DrawingBoardData_Snow.BP_DrawingBoardData_Snow_C|GetSnowThickness (LocalVariables|GetSnowData)) :!class /Script/Engine.MaterialInstanceDynamic)
        (Rendering|Material|SetScalarParameterValue _output_get_2 "ShadowSoftness" (Variables|/InteractiveWorld/Blueprints/DataAssets/BP_DrawingBoardData_Snow.BP_DrawingBoardData_Snow_C|GetShadowSoftness (LocalVariables|GetSnowData)) :!class /Script/Engine.MaterialInstanceDynamic)
        (Rendering|Material|SetScalarParameterValue _output_get_2 "ShadowIntensity" (Variables|/InteractiveWorld/Blueprints/DataAssets/BP_DrawingBoardData_Snow.BP_DrawingBoardData_Snow_C|GetSelfShadowIntensity (LocalVariables|GetSnowData)) :!class /Script/Engine.MaterialInstanceDynamic)
        (Rendering|Material|SetScalarParameterValue _output_get_2 "WorldSize" (.x (Variables|Default|GetCanvasWorldSize)) :!class /Script/Engine.MaterialInstanceDynamic)
        (Rendering|Material|SetScalarParameterValue _output_get_2 "FallTime" (Variables|/InteractiveWorld/Blueprints/DataAssets/BP_DrawingBoardData_Snow.BP_DrawingBoardData_Snow_C|GetFreshSnowFallTime (LocalVariables|GetSnowData)) :!class /Script/Engine.MaterialInstanceDynamic)))
    (:then_3
      (Rendering|Material|SetVectorParameterValue _boardmpc (Utilities|Name|MakeLiteralName "SnowSurfaceColor") (Variables|/InteractiveWorld/Blueprints/DataAssets/BP_DrawingBoardData_Snow.BP_DrawingBoardData_Snow_C|GetSnowSubSurfaceColor (LocalVariables|GetSnowData)) :!class /Script/Engine.KismetMaterialLibrary)
      (Rendering|Material|SetScalarParameterValue _boardmpc (Utilities|Name|MakeLiteralName "SnowThickness") (Variables|/InteractiveWorld/Blueprints/DataAssets/BP_DrawingBoardData_Snow.BP_DrawingBoardData_Snow_C|GetSnowThickness (LocalVariables|GetSnowData)) :!class /Script/Engine.KismetMaterialLibrary)
      (Rendering|Material|SetScalarParameterValue _boardmpc (Utilities|Name|MakeLiteralName "LowQualityBool") (Math|Float|SelectFloat 1.0 0.0 (Variables|Default|GetLowQuality)) :!class /Script/Engine.KismetMaterialLibrary))
    (:then_4
      (Variables|Default|SetCurrent (Variables|/InteractiveWorld/Blueprints/DataAssets/BP_DrawingBoardData_Snow.BP_DrawingBoardData_Snow_C|GetSimulateRT (LocalVariables|GetSnowData)))
      (Variables|Default|SetPrevious (Variables|/InteractiveWorld/Blueprints/DataAssets/BP_DrawingBoardData_Snow.BP_DrawingBoardData_Snow_C|GetSaveRT (LocalVariables|GetSnowData)))
      (Rendering|ClearRenderTarget2D (Variables|Default|GetCurrent) "(R=1.000000,G=0.000000,B=1.000000,A=1.000000)")
      (Rendering|ClearRenderTarget2D (Variables|Default|GetPrevious) "(R=1.000000,G=0.000000,B=1.000000,A=1.000000)")
      (Rendering|ClearRenderTarget2D (Variables|Default|GetOutput%20RT) "(R=1.000000,G=1.000000,B=1.000000,A=1.000000)"))))

(fn SwitchRTs
  (LocalVariables|SetTempRT (Variables|Default|GetCurrent))
  (Variables|Default|SetCurrent (Variables|Default|GetPrevious))
  (Variables|Default|SetPrevious (LocalVariables|GetTempRT)))