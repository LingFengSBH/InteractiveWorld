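; Shape brush that stamps a sphere or box footprint onto a drawing board's render target, apparently for snow interaction.
; BeginPlay sizes it from Bounds and creates a dynamic instance of the matching ray-tracing material.
; UpdateDrawInfo feeds rotation axes, extents and height to the material, which DrawonRT draws at a position and height interpolated between previous and current values.
; A debug event visualizes the shape.
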(event Custom|DrawBebugShape
  (bind _returnvalue (Transformation|GetWorldTransform))
  (bind _bounds (Variables|ShapeSettings|GetBounds))
  (bind _returnvalue_2 (/ _bounds "2.000000,2.000000,2.000000"))
  (switch Utilities|FlowControl|Switch|SwitchonE_BrushShape (Variables|ShapeSettings|GetShape)
    (:NewEnumerator0
      (Rendering|Debug|DrawDebugSphere (.location _returnvalue) (.X (Math|Vector|BreakVector _returnvalue_2)) 12 "(R=1.000000,G=0.000000,B=0.000000,A=1.000000)" 3.0 2.0))
    (:NewEnumerator1
      (Rendering|Debug|DrawDebugBox (.location _returnvalue) _returnvalue_2 "(R=1.000000,G=0.000000,B=0.000000,A=1.000000)" (.rotation _returnvalue) 3.0 2.0))))

(event EventBeginPlay
  (CallFunction|ResetBounds (Variables|ShapeSettings|GetBounds))
  (bind _returnvalue (Rendering|Material|CreateDynamicMaterialInstance (Utilities|Select :Index (Variables|ShapeSettings|GetShape) :NewEnumerator0 "/InteractiveWorld/Materials/BrushMaterials/RayTrace/M_RayTracing_Sphere.M_RayTracing_Sphere" :NewEnumerator1 "/InteractiveWorld/Materials/BrushMaterials/RayTrace/M_RayTracing_Box.M_RayTracing_Box") "None" "None" :!class /Script/Engine.KismetMaterialLibrary))
  (Variables|Default|SetShapeMaterial _returnvalue))

(event EventDrawonRT
  (params (DrawingBoard :type World%20Drawing%20Board%20Object%20Reference) (CanvasDrawOn :type Canvas%20Object%20Reference) (CanvasSize :type Vector%202D%20Structure) (InterpolateRate :type Float%20%28single-precision%29) (DrawTimes :type Integer))
  (bind _size (Variables|Default|GetSize))
  (bind _size_2 (Variables|Default|GetSize))
  (bind _shapematerial (Variables|Default|GetShapeMaterial))
  (bind _previoust (Variables|Default|GetPreviousT))
  (bind _currentt (Variables|Default|GetCurrentT))
  (bind _returnvalue (Math|Vector|Lerp(Vector) (.location _previoust) (.location _currentt) InterpolateRate))
  (bind _returnvalue_2 (Math|Conversions|ToVector2D(Vector) _returnvalue))
  (bind (_outscreenposition _outscreensize) (Class|WorldDrawingBoard|WorldtoCanvasBrush DrawingBoard _returnvalue_2 _size 0.0))
  (Rendering|Material|SetVectorParameterValue _shapematerial "SizeHeight" (Math|Color|MakeColor (.x _size_2) (.y _size_2) (Math|Float|Lerp (Variables|Default|GetPreviousHeight) (Variables|Default|GetHeight) InterpolateRate)) :!class /Script/Engine.MaterialInstanceDynamic)
  (Rendering|Material|SetScalarParameterValue _shapematerial "SnowThickness" (Class|WorldDrawingBoard|GetInteractHeight DrawingBoard) :!class /Script/Engine.MaterialInstanceDynamic)
  (Canvas|DrawMaterial :self CanvasDrawOn :RenderMaterial _shapematerial :ScreenPosition _outscreenposition :ScreenSize _outscreensize :CoordinateSize "(X=1.000000,Y=1.000000)" :PivotPoint "(X=0.500000,Y=0.500000)"))

(fn UpdateDrawInfo
  (bind _returnvalue (Transformation|GetWorldTransform))
  (bind _shapematerial (Variables|Default|GetShapeMaterial))
  (bind _size (Variables|Default|GetSize))
  (bind _bounds (Variables|ShapeSettings|GetBounds))
  (bind _returnvalue_2 (Math|Vector|GetForwardVector (.rotation _returnvalue)))
  (bind _returnvalue_3 (Math|Vector|GetRightVector (.rotation _returnvalue)))
  (bind _returnvalue_4 (Math|Vector|GetUpVector (.rotation _returnvalue)))
  (bind _returnvalue_5 (|CallParentFunction))
  (Rendering|Material|SetVectorParameterValue _shapematerial "AxisX" (Utilities|Struct|MakeLinearColor (.x _returnvalue_2) (.y _returnvalue_2) (.z _returnvalue_2) (.x _bounds)) :!class /Script/Engine.MaterialInstanceDynamic)
  (Rendering|Material|SetVectorParameterValue _shapematerial "AxisY" (Utilities|Struct|MakeLinearColor (.x _returnvalue_3) (.y _returnvalue_3) (.z _returnvalue_3) (.y _bounds)) :!class /Script/Engine.MaterialInstanceDynamic)
  (Rendering|Material|SetVectorParameterValue _shapematerial "AxisZ" (Utilities|Struct|MakeLinearColor (.x _returnvalue_4) (.y _returnvalue_4) (.z _returnvalue_4) (.z _bounds)) :!class /Script/Engine.MaterialInstanceDynamic)
  (Rendering|Material|SetVectorParameterValue _shapematerial "SizeHeight" (Math|Color|MakeColor (.x _size) (.y _size) (Variables|Default|GetHeight)) :!class /Script/Engine.MaterialInstanceDynamic)
  (return _returnvalue_5))

(fn ResetBounds
  (params (NewBounds :type Vector))
  (bind _returnvalue (Math|Vector|VectorLength NewBounds))
  (Variables|ShapeSettings|SetBounds NewBounds)
  (Variables|Default|SetSize (Math|Vector2D|MakeVector2D _returnvalue _returnvalue))
  (Variables|Default|SetInteractDistance (+ (/ _returnvalue 2.0) (Variables|Default|GetSnowHeight))))