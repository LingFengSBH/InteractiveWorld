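; Fluid brush Blueprint that stamps a force material onto a drawing board's render target canvas.
; On BeginPlay it creates a dynamic instance of M_FluidForce with the brush mask.
; Each draw sets the material's Velocity from either fixed forward strength or frame-to-frame movement normalized by canvas world size.
; It then draws the stamp at the interpolated position between previous and current transforms, rotated to the brush's forward yaw.
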(event EventBeginPlay
  (|CallParentFunction)
  (bind _returnvalue (Rendering|Material|CreateDynamicMaterialInstance "/InteractiveWorld/Materials/BrushMaterials/M_FluidForce.M_FluidForce" "None" "None" :!class /Script/Engine.KismetMaterialLibrary))
  (bind _output_get (Variables|Default|SetTurbulentMaterial _returnvalue))
  (Rendering|Material|SetTextureParameterValue _output_get "Mask" (Variables|Default|GetMask)))

(event EventTick
  (params (DeltaSeconds :type Float%20%28single-precision%29))
  (|CallParentFunction DeltaSeconds) ; 此节点被禁用，将不会被调用。\n从引脚连出引线来编译功能。
)

(event EventDrawonRT
  (params (DrawingBoard :type World%20Drawing%20Board%20Object%20Reference) (CanvasDrawOn :type Canvas%20Object%20Reference) (CanvasSize :type Vector%202D%20Structure) (InterpolateRate :type Float%20%28single-precision%29) (DrawTimes :type Integer))
  (bind _size (Variables|Default|GetSize))
  (bind _turbulentmaterial (Variables|Default|GetTurbulentMaterial))
  (bind _canvasworldsize (Variables|/Script/InteractiveWorld.WorldDrawingBoard|GetCanvasWorldSize DrawingBoard))
  (bind _currentt (Variables|Default|GetCurrentT))
  (bind _previoust (Variables|Default|GetPreviousT))
  (bind (_x _y) (Math|Vector2D|BreakVector2D _canvasworldsize))
  (bind _returnvalue (Math|Vector|GetForwardVector (.rotation _currentt)))
  (bind _returnvalue_2 (Math|Vector|Lerp(Vector) (.location _previoust) (.location _currentt) InterpolateRate))
  (bind _returnvalue_3 (Math|Rotator|MakeRotfromZX (Math|Vector|MakeVector 0.0 0.0 1.0) _returnvalue))
  (bind _returnvalue_4 (Math|Conversions|ToVector2D(Vector) _returnvalue_2))
  (bind _yaw (Math|Rotator|BreakRotator _returnvalue_3))
  (bind (_outscreenposition _outscreensize _outscreenrotation) (Class|WorldDrawingBoard|WorldtoCanvasBrush DrawingBoard _returnvalue_4 _size _yaw))
  (if (Class|InteractBrush|GetLastDrawSucceed)
    (Rendering|Material|SetVectorParameterValue _turbulentmaterial "Velocity" (Math|Conversions|ToLinearColor(Vector) (Math|Vector|SelectVector (* _returnvalue (Variables|Default|GetFixedVelocityStrength)) (/ (/ (- (.location _currentt) (.location _previoust)) (Utilities|Time|GetWorldDeltaSeconds)) (Math|Vector|MakeVector _x _y 1.0)) (Variables|Default|GetFixedVelocity))) :!class /Script/Engine.MaterialInstanceDynamic)
    (Canvas|DrawMaterial :self CanvasDrawOn :RenderMaterial _turbulentmaterial :ScreenPosition _outscreenposition :ScreenSize _outscreensize :CoordinateSize "(X=1.000000,Y=1.000000)" :Rotation _outscreenrotation :PivotPoint "(X=0.500000,Y=0.500000)")))