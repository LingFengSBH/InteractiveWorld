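; Line-trace brush that draws patterned wheel tracks with depth onto a drawing board's render target as the wheel moves.
; Each draw converts previous and current transforms to canvas space, deriving pattern UVs from wheel roll and depth from trace height minus radius.
; When heading changes enough, intersecting the two axle lines gives a turn center for a full-canvas curved-arc material.
; Otherwise it draws a straight, rotated material quad between both points.
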(event EventBeginPlay
  (|CallParentFunction)
  (bind _returnvalue (Rendering|Material|CreateDynamicMaterialInstance "/InteractiveWorld/Materials/BrushMaterials/Wheel/M_CurveWheel.M_CurveWheel" "None" "None" :!class /Script/Engine.KismetMaterialLibrary))
  (bind _output_get (Variables|Default|SetWheelMat _returnvalue))
  (Rendering|Material|SetTextureParameterValue _output_get "WhellPattern" (Variables|WheelSetting|GetWheelPattern))
  (bind _returnvalue_2 (Rendering|Material|CreateDynamicMaterialInstance "/InteractiveWorld/Materials/BrushMaterials/Wheel/M_Wheel.M_Wheel" "None" "None" :!class /Script/Engine.KismetMaterialLibrary))
  (bind _output_get_2 (Variables|Default|SetSimpleWheelMat _returnvalue_2))
  (Rendering|Material|SetTextureParameterValue _output_get_2 "WhellPattern" (Variables|WheelSetting|GetWheelPattern)))

(event EventDrawonRT
  (params (DrawingBoard :type World%20Drawing%20Board%20Object%20Reference) (CanvasDrawOn :type Canvas%20Object%20Reference) (CanvasSize :type Vector%202D%20Structure) (InterpolateRate :type Float%20%28single-precision%29) (DrawTimes :type Integer))
  (if (Class|InteractBrush|GetLastDrawSucceed)
    (bind _s_whell (CallFunction|CreateWheelInfo DrawingBoard CanvasSize))
    (bind (_success _center) (CallFunction|CalculateWheel _s_whell))
    (if _success
      (CallFunction|DrawCurveWheel _center _s_whell CanvasDrawOn CanvasSize)
      (else
        (CallFunction|DrawSimpleWheel CanvasDrawOn _s_whell CanvasSize)))))

(fn SolveAngle
  (params (Previous :type Float%20%28double-precision%29) (Current :type Float%20%28double-precision%29))
  (if (> Previous Current)
    (if (> (- Previous Current) 1.8e+02)
      (return (/ (- Previous 3.6e+02) 3.6e+02) (/ Current 3.6e+02))
      (else
        (return (/ (- Previous 1.8e+02) 3.6e+02) (/ (- Current 1.8e+02) 3.6e+02))))
    (elif (> (- Current Previous) 1.8e+02)
      (return (/ (+ (- Previous 1.8e+02) 3.6e+02) 3.6e+02) (/ (- Current 1.8e+02) 3.6e+02))
      (else
        (return (/ Previous 3.6e+02) (/ Current 3.6e+02))))))

(fn CalculateWheel
  (params (S_Whell :type S%20Whell%20Structure%20%28by%20ref%29))
  (bind (_lastlocation _currentlocation _lastrotation _currentrotation) (Utilities|Struct|BreakS_Whell S_Whell))
  (bind (_x _y) (Math|Vector2D|BreakVector2D _lastlocation))
  (bind _returnvalue (Class|KismetMathLibrary|GetRotated2D "(X=0.000000,Y=1.000000)" _currentrotation))
  (bind _returnvalue_2 (Class|KismetMathLibrary|GetRotated2D "(X=0.000000,Y=1.000000)" _lastrotation))
  (bind (_x_2 _y_2) (Math|Vector2D|BreakVector2D _currentlocation))
  (bind (_x_3 _y_3) (Math|Vector2D|BreakVector2D _returnvalue_2))
  (bind (_x_4 _y_4) (Math|Vector2D|BreakVector2D _returnvalue))
  (bind _returnvalue_3 (/ _y_4 _x_4))
  (bind _returnvalue_4 (/ _y_3 _x_3))
  (if (> (Math|Float|Absolute(Float) (- _lastrotation _currentrotation)) 3.0)
    (LocalVariables|SetX (/ (- (+ (- _y_2 _y) (* _x _returnvalue_4)) (* _x_2 _returnvalue_3)) (- _returnvalue_4 _returnvalue_3)))
    (return true (Math|Vector2D|MakeVector2D (LocalVariables|GetX) (+ _y (* _returnvalue_4 (- (LocalVariables|GetX) _x)))))
    (else
      (return false ""))))

(fn CreateWheelInfo
  (params (DrawingBoard :type World%20Drawing%20Board%20Object%20Reference) (CanvasSize :type Vector%202D%20Structure))
  (bind _returnvalue (Class|WorldDrawingBoard|GetInteractHeight DrawingBoard))
  (bind _previoust (Variables|Default|GetPreviousT))
  (bind _currentt (Variables|Default|GetCurrentT))
  (bind _wheelradius (Variables|WheelSetting|GetWheelRadius))
  (bind (_location _rotation) (Math|Transform|BreakTransform _currentt))
  (bind (_location_2 _rotation_2) (Math|Transform|BreakTransform _previoust))
  (return (Utilities|Struct|MakeS_Whell (Class|WorldDrawingBoard|WorldtoCanvasUV DrawingBoard (Math|Conversions|ToVector2D(Vector) _location_2)) (Class|WorldDrawingBoard|WorldtoCanvasUV DrawingBoard (Math|Conversions|ToVector2D(Vector) _location)) (Class|WorldDrawingBoard|WorldtoCanvasRotation DrawingBoard (.Yaw (Math|Rotator|BreakRotator (Math|Rotator|MakeRotfromZY (Math|Vector|MakeVector 0.0 0.0 1.0) (Math|Vector|GetForwardVector _rotation_2))))) (Class|WorldDrawingBoard|WorldtoCanvasRotation DrawingBoard (.Yaw (Math|Rotator|BreakRotator (Math|Rotator|MakeRotfromZY (Math|Vector|MakeVector 0.0 0.0 1.0) (Math|Vector|GetForwardVector _rotation))))) (CallFunction|WheelUV _rotation_2 _rotation) (/ (.x (Class|WorldDrawingBoard|WorldtoCanvasSize DrawingBoard (Variables|Default|GetSize))) (.X (Math|Vector2D|BreakVector2D CanvasSize))) (/ (- (Variables|Default|GetPreviousTraceHeight) _wheelradius) _returnvalue) (/ (- (Variables|Default|GetTraceHeight) _wheelradius) _returnvalue))))

(fn DrawSimpleWheel
  (params (Canvas :type Canvas%20Object%20Reference) (S_Whell :type S%20Whell%20Structure%20%28by%20ref%29) (CanvasSize :type Vector%202D%20Structure))
  (bind (_lastlocation _currentlocation _lastrotation _currentrotation _uvrange _width _lastheight _currentheight) (Utilities|Struct|BreakS_Whell S_Whell))
  (bind _simplewheelmat (Variables|Default|GetSimpleWheelMat))
  (bind (_moverotation _outlength _foward) (CallFunction|MoveDirection _lastlocation _currentlocation _currentrotation))
  (bind (_x _y) (Math|Vector2D|BreakVector2D _uvrange))
  (LocalVariables|SetMoveFoward _foward)
  (LocalVariables|SetMoveRotation _moverotation)
  (LocalVariables|SetMoveLength _outlength)
  (Rendering|Material|SetVectorParameterValue _simplewheelmat "UVDepth" (Math|Color|MakeColor (.X (Math|Vector2D|BreakVector2D (select (LocalVariables|GetMoveFoward) _uvrange (Math|Vector2D|MakeVector2D _y _x)))) (.Y (Math|Vector2D|BreakVector2D (select (LocalVariables|GetMoveFoward) _uvrange (Math|Vector2D|MakeVector2D _y _x)))) _lastheight _currentheight) :!class /Script/Engine.MaterialInstanceDynamic)
  (Canvas|DrawMaterial :self Canvas :RenderMaterial _simplewheelmat :ScreenPosition (* (- (/ (+ _lastlocation _currentlocation) "(X=2.000000,Y=2.000000)") (/ (Math|Vector2D|MakeVector2D _width (LocalVariables|GetMoveLength)) "(X=2.000000,Y=2.000000)")) CanvasSize) :ScreenSize (* (Math|Vector2D|MakeVector2D _width (LocalVariables|GetMoveLength)) CanvasSize) :CoordinateSize "(X=1.000000,Y=1.000000)" :Rotation (Math|Float|SelectFloat (LocalVariables|GetMoveRotation) (+ (LocalVariables|GetMoveRotation) 1.8e+02) (LocalVariables|GetMoveFoward)) :PivotPoint "(X=0.500000,Y=0.500000)"))

(fn DrawCurveWheel
  (params (Center :type Vector%202D%20Structure) (S_Whell :type S%20Whell%20Structure%20%28by%20ref%29) (Canvas :type Canvas%20Object%20Reference) (CanvasSize :type Vector%202D%20Structure))
  (bind (_lastlocation _currentlocation _lastrotation _currentrotation _uvrange _width _lastheight _currentheight) (Utilities|Struct|BreakS_Whell S_Whell))
  (bind (_x _y) (Math|Vector2D|BreakVector2D Center))
  (bind _wheelmat (Variables|Default|GetWheelMat))
  (bind _returnvalue (Math|Vector|Distance2D(Vector) Center _currentlocation))
  (bind _returnvalue_2 (Math|Vector|Distance2D(Vector) Center _lastlocation))
  (bind (_x_2 _y_2) (Math|Vector2D|BreakVector2D _uvrange))
  (bind _returnvalue_3 (Class|KismetMathLibrary|GetRotated2D "(X=1.000000,Y=0.000000)" _lastrotation))
  (bind _returnvalue_4 (- _currentlocation _lastlocation))
  (bind _returnvalue_5 (* _width 0.5))
  (bind _returnvalue_6 (Math|Vector2D|DotProduct(2D) _returnvalue_4 _returnvalue_3))
  (bind _returnvalue_7 (> _returnvalue_6 0.0))
  (bind _returnvalue_8 (Math|Float|SelectFloat 0.0 1.8e+02 _returnvalue_7))
  (bind (_a _b) (CallFunction|SolveAngle (+ _lastrotation _returnvalue_8) (+ _currentrotation _returnvalue_8)))
  (Rendering|Material|SetVectorParameterValue _wheelmat "CenterAngle" (Utilities|Struct|MakeLinearColor _x _y _a _b) :!class /Script/Engine.MaterialInstanceDynamic)
  (Rendering|Material|SetVectorParameterValue _wheelmat "Radius" (Utilities|Struct|MakeLinearColor (- _returnvalue_2 _returnvalue_5) (+ _returnvalue_5 _returnvalue_2) (- _returnvalue _returnvalue_5) (+ _returnvalue_5 _returnvalue)) :!class /Script/Engine.MaterialInstanceDynamic)
  (Rendering|Material|SetVectorParameterValue _wheelmat "UVDepth" (Math|Color|MakeColor _x_2 _y_2 _lastheight _currentheight) :!class /Script/Engine.MaterialInstanceDynamic)
  (Canvas|DrawMaterial :self Canvas :RenderMaterial _wheelmat :ScreenSize CanvasSize :CoordinateSize "(X=1.000000,Y=1.000000)" :PivotPoint "(X=0.500000,Y=0.500000)"))

(fn WheelUV
  (params (InRot :type Rotator) (InRot2 :type Rotator))
  (bind _roll (Math|Rotator|BreakRotator InRot))
  (bind _roll_2 (Math|Rotator|BreakRotator InRot2))
  (bind _returnvalue (- _roll _roll_2))
  (bind _returnvalue_2 (Math|Float|Absolute(Float) _returnvalue))
  (return (/ (select (> _returnvalue_2 1.8e+02) (Math|Vector2D|MakeVector2D _roll (+ _roll (* (Math|Float|Sign(Float) _returnvalue) (- 3.6e+02 _returnvalue_2)))) (Math|Vector2D|MakeVector2D _roll _roll_2)) "(X=360.000000,Y=360.000000)")))

(fn MoveDirection
  (params (PreviousLocation :type Vector%202D%20Structure) (CurrentLocation :type Vector%202D%20Structure) (Rotation :type Float%20%28double-precision%29))
  (bind _returnvalue (- CurrentLocation PreviousLocation))
  (bind (_outdir _outlength) (Class|KismetMathLibrary|ToDirectionandLength2D _returnvalue))
  (bind _returnvalue_2 (Class|KismetMathLibrary|DegAtan2 (.y _outdir) (.x _outdir)))
  (bind _returnvalue_3 (+ _returnvalue_2 -9e+01))
  (return _returnvalue_3 _outlength (> (- _returnvalue_3 Rotation) 0.0)))