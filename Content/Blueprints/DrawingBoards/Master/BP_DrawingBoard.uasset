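; Master drawing board Blueprint that maintains a world-space render-target canvas following the player pawn, a target actor or its own location.
; A data asset supplies the output target and world size, and location updates can snap to pixels.
; Helper functions reproject the previous target into the current one through a material using canvas movement, rotation and scale deltas.
; After simulation it publishes canvas position and size to a Material Parameter Collection.
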(event EventBeginPlay
  (bind _returnvalue (Rendering|Material|CreateDynamicMaterialInstance "/InteractiveWorld/Materials/DrawingBoardMaterials/CommonSimulateMat/M_RenderPreviousToCurrent.M_RenderPreviousToCurrent" "None" "None" :!class /Script/Engine.KismetMaterialLibrary))
  (Variables|Default|SetPreviousToCurrent _returnvalue)
  (CallFunction|InitializewithDataAsset (Variables|Data|GetDataAsset))
  (Rendering|ClearRenderTarget2D (Variables|Default|GetOutput%20RT))
  (CallFunction|UpdateSimulateLocation true 1.0)
  (if (Variables|Debug|GetDebugOutputRT)
    (CallFunction|AddRTDebugUI)))

(event EventEndPlay
  (params (EndPlayReason :type EEndPlayReason%20Enum :default "Destroyed"))
  (bind _output_rt (Variables|Default|GetOutput%20RT))
  (|CallParentFunction EndPlayReason)
  (switch Utilities|FlowControl|Switch|SwitchonEEndPlayReason EndPlayReason
    (:LevelTransition
      _)
    (:EndPlayInEditor
      _)
    (:Quit
      _))
  (Rendering|ClearRenderTarget2D _output_rt (Variables|/Script/Engine.TextureRenderTarget2D|GetClearColor _output_rt)))

(event EventUpdateDrawingBoardState
  (CallFunction|UpdateSimulateLocation true 1.0))

(event EventPreSimulate)

(event EventPostSimulate
  (Material|SetMPC))

(fn ConstructionScript)

(fn CurrenttoPreviousMatrix
  (bind _previouscanvasworldyaw (Variables|Default|GetPreviousCanvasWorldYaw))
  (bind _canvasworldyaw (Variables|Default|GetCanvasWorldYaw))
  (bind _previouscanvasworldsize (Variables|Default|GetPreviousCanvasWorldSize))
  (bind _canvasworldsize (Variables|Default|GetCanvasWorldSize))
  (bind _returnvalue (- _canvasworldyaw _previouscanvasworldyaw))
  (bind _returnvalue_2 (/ _canvasworldsize _previouscanvasworldsize))
  (return (Class|KismetMathLibrary|GetRotated2D (* _returnvalue_2 "(X=1.000000,Y=0.000000)") _returnvalue) (Class|KismetMathLibrary|GetRotated2D (* _returnvalue_2 "(X=0.000000,Y=1.000000)") _returnvalue) (/ (Class|KismetMathLibrary|GetRotated2D (- (Variables|Default|GetCanvasWorldLocation) (Variables|Default|GetPreviousCanvasWorldLocation)) (* (Variables|Default|GetPreviousCanvasWorldYaw) -1.0)) (Variables|Default|GetPreviousCanvasWorldSize))))

(fn SetCurrenttoPreviousMaterialParam
  (params (Target :type Material%20Instance%20Dynamic%20Object%20Reference))
  (bind (_xaxis _yaxis _offset) (CallFunction|CurrenttoPreviousMatrix))
  (Rendering|Material|SetVectorParameterValue Target "AxisXY" (Utilities|Struct|MakeLinearColor (.x _xaxis) (.y _xaxis) (.x _yaxis) (.y _yaxis)) :!class /Script/Engine.MaterialInstanceDynamic)
  (Rendering|Material|SetVectorParameterValue Target "Offset" (Utilities|Struct|MakeLinearColor (.x _offset) (.y _offset) 0.0 0.0) :!class /Script/Engine.MaterialInstanceDynamic))

(fn RenderPrevioustoCurrent
  (params (RT_Previous :type Texture%20Render%20Target%202D%20Object%20Reference) (RT_Current :type Texture%20Render%20Target%202D%20Object%20Reference) (DefaultColor :type Linear%20Color%20Structure))
  (bind _previoustocurrent (Variables|Default|GetPreviousToCurrent))
  (Rendering|Material|SetVectorParameterValue _previoustocurrent "DefaultColor" DefaultColor :!class /Script/Engine.MaterialInstanceDynamic)
  (Material|SetCurrenttoPreviousMaterialParam _previoustocurrent)
  (Rendering|Material|SetTextureParameterValue _previoustocurrent "Previous" RT_Previous)
  (Rendering|DrawMaterialtoRenderTarget RT_Current _previoustocurrent))

(fn UpdateLocationtoPlayer
  (bind _returnvalue (Game|Player|GetPlayerPawn 0))
  ;[1 1 1] Use "Update Simulate Location"instead
  (Utilities|IsValid _returnvalue
    (:Is%20Valid
      (Class|WorldDrawingBoard|SetCanvasWorldLocation (Math|Conversions|ToVector2D(Vector) (Transformation|GetActorLocation _returnvalue)) true 1.0))))

(fn SetMPC
  (bind _boardmpc (Variables|Material|GetBoardMPC))
  (bind _canvasworldsize (Variables|Default|GetCanvasWorldSize))
  (bind _canvasworldlocation (Variables|Default|GetCanvasWorldLocation))
  (bind _returnvalue (Math|Color|MakeColor (.x _canvasworldlocation) (.y _canvasworldlocation) (.x _canvasworldsize) (.y _canvasworldsize)))
  (Utilities|IsValid _boardmpc
    (:Is%20Valid
      (Rendering|Material|SetVectorParameterValue _boardmpc (Utilities|Name|MakeLiteralName "PositionSize") _returnvalue :!class /Script/Engine.KismetMaterialLibrary)
      (Variables|Material|SetRenderLocationSize _returnvalue))))

(fn CheckDataAssetType
  (bind _dataassetclass (Variables|Default|GetDataAssetClass))
  (if (== (Utilities|GetClass (Variables|Data|GetDataAsset)) _dataassetclass)
    (return true)
    (else
      (Development|PrintText (Utilities|Text|FormatText "{Object}:DrawingBoard has wrong DataAsset type,Expected:{Class}" (Utilities|GetDisplayName self) (Utilities|GetClassDisplayName _dataassetclass)))
      (return false))))

(fn InitializewithDataAsset
  (params (Data :type BP%20Drawing%20Board%20Data%20Object%20Reference))
  (bind _outputrt (Variables|/InteractiveWorld/Blueprints/DataAssets/Master/BP_DrawingBoardData.BP_DrawingBoardData_C|GetOutputRT Data))
  (bind _simulateworldsize (Variables|/InteractiveWorld/Blueprints/DataAssets/Master/BP_DrawingBoardData.BP_DrawingBoardData_C|GetSimulateWorldSize Data))
  (Variables|Default|SetOutput%20RT _outputrt)
  (bind _output_get (Variables|Default|SetRTSize (Math|Vector2D|MakeVector2D (Math|Conversions|ToFloat(Integer) (Variables|/Script/Engine.TextureRenderTarget2D|GetSizeX _outputrt)) (Math|Conversions|ToFloat(Integer) (Variables|/Script/Engine.TextureRenderTarget2D|GetSizeY _outputrt)))))
  (Variables|Default|SetPreviousRTSize _output_get)
  (bind _output_get_2 (Variables|Default|SetCanvasWorldSize (Math|Vector2D|MakeVector2D _simulateworldsize _simulateworldsize)))
  (Variables|Default|SetPreviousCanvasWorldSize _output_get_2)
  (Material|SetMPC)
  (bind _output_get_3 (Variables|Default|SetPixelWorldSize (/ _output_get_2 _output_get)))
  (Variables|Default|SetPreviousPixelWorldSize _output_get_3)
  (bind _returnvalue (CallFunction|CheckDataAssetType))
  (if _returnvalue
    _))

(fn SetMaterialCanvasParameters
  (params (Target :type Material%20Instance%20Dynamic%20Object%20Reference))
  (Rendering|Material|SetScalarParameterValue Target "Resolution" (.x (Variables|Default|GetRTSize)) :!class /Script/Engine.MaterialInstanceDynamic)
  (Rendering|Material|SetScalarParameterValue Target "WorldSize" (Variables|/InteractiveWorld/Blueprints/DataAssets/Master/BP_DrawingBoardData.BP_DrawingBoardData_C|GetSimulateWorldSize (Variables|Data|GetDataAsset)) :!class /Script/Engine.MaterialInstanceDynamic))

(fn AddRTDebugUI
  (bind _self self)
  (bind _foundwidgets (Widget|GetAllWidgetsOfClass "/InteractiveWorld/EditorWidgets/DebugUI/UI_DrawingBoardDebugPanel.UI_DrawingBoardDebugPanel_C" true))
  (if (> (Utilities|Array|Length _foundwidgets) 0)
    (Default|AddDebugUI (Utilities|Array|Get(acopy) _foundwidgets) _self)
    (else
      (bind _returnvalue (UserInterface|CreateWidget "/InteractiveWorld/EditorWidgets/DebugUI/UI_DrawingBoardDebugPanel.UI_DrawingBoardDebugPanel_C"))
      (UserInterface|Viewport|AddtoViewport _returnvalue 0)
      (Default|AddDebugUI _returnvalue _self))))

(fn GetSimulateLocation
  (bind _returnvalue (Game|Player|GetPlayerPawn 0))
  (bind _targetactor (Variables|SimulateFollowing|GetTargetActor))
  (switch Utilities|FlowControl|Switch|SwitchonE_SimulateLocation (Variables|SimulateFollowing|GetFollowMode)
    (:NewEnumerator0
      (Utilities|IsValid _returnvalue
        (:Is%20Valid
          (return (Transformation|GetActorLocation _returnvalue)))
        (:Is%20Not%20Valid
          _)))
    (:NewEnumerator1
      (Utilities|IsValid _targetactor
        (:Is%20Valid
          (return (Transformation|GetActorLocation _targetactor)))
        (:Is%20Not%20Valid
          _)))
    (:NewEnumerator2
      _))
  (return (Transformation|GetActorLocation)))

(fn UpdateSimulateLocation
  (params (bPixelAligned :type Boolean) (PixelSizeScale :type Float%20%28single-precision%29))
  ;[1 1 1] Where this DrawingBoard  simulate in.
  (bind _returnvalue (CallFunction|GetSimulateLocation))
  (Class|WorldDrawingBoard|SetCanvasWorldLocation (Math|Conversions|ToVector2D(Vector) _returnvalue) bPixelAligned PixelSizeScale))