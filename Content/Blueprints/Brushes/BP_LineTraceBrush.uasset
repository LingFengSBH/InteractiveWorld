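; BP_LineTraceBrush is a render target brush variant that derives its draw info from a vertical line trace against world static objects.
; UpdateDrawInfo traces through the brush's current location, from MaxTrace above to MaxTrace below.
; A hit stores the impact point and the surface's offset-adjusted depth below the brush, clamped at zero, while a miss zeroes the height.
; It keeps the previous height and returns whether it hit.
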(event EventBeginPlay)

(event EventTick
  (params (DeltaSeconds :type Float%20%28single-precision%29)))

(event EventDrawonRT
  (params (DrawingBoard :type World%20Drawing%20Board%20Object%20Reference) (CanvasDrawOn :type Canvas%20Object%20Reference) (CanvasSize :type Vector%202D%20Structure) (InterpolateRate :type Float%20%28single-precision%29) (DrawTimes :type Integer)))

(fn UpdateDrawInfo
  (bind _maxtrace (Variables|LineTrace|GetMaxTrace))
  (bind _currentt (Variables|Default|GetCurrentT))
  (bind _location (Math|Transform|BreakTransform _currentt))
  (Variables|LineTrace|SetPreviousTraceHeight (Variables|LineTrace|GetTraceHeight))
  (bind (_outhit _returnvalue) (Collision|LineTraceForObjects (+ _location (Math|Vector|MakeVector 0.0 0.0 (Variables|LineTrace|GetMaxTrace))) (- _location (Math|Vector|MakeVector 0.0 0.0 _maxtrace)) (Utilities|Array|MakeArray "ObjectTypeQuery1") false 0 "None"))
  (if _returnvalue
    (Variables|LineTrace|SetTraceHeight (Math|Float|Max(Float) (+ (- (.Distance (Collision|BreakHitResult _outhit)) _maxtrace) (Variables|LineTrace|GetTraceOffset)) 0.0))
    (Variables|LineTrace|SetTracePoint (.ImpactPoint (Collision|BreakHitResult _outhit)))
    (return true)
    (else
      (Variables|LineTrace|SetTraceHeight 0.0)
      (return false))))