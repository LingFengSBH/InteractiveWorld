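; BP_Brush_MudStep is a brush that stamps a texture, by its name a mud footstep, onto a drawing board's render target.
; DrawonRT converts the brush's location, size and forward-vector yaw into canvas space through the DrawingBoard, then draws the texture additively around a centered pivot.
; MirrorFlip mirrors the stamp horizontally through a negative coordinate size.
; UpdateDrawInfo always returns true.
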(event EventBeginPlay
  (|CallParentFunction) ; This node is disabled and will not be called.\nDrag off pins to build functionality.
)

(event EventTick
  (params (DeltaSeconds :type Float%20%28single-precision%29))
  (|CallParentFunction DeltaSeconds) ; This node is disabled and will not be called.\nDrag off pins to build functionality.
)

(event EventDrawonRT
  (params (DrawingBoard :type World%20Drawing%20Board%20Object%20Reference) (CanvasDrawOn :type Canvas%20Object%20Reference) (CanvasSize :type Vector%202D%20Structure) (InterpolateRate :type Float%20%28single-precision%29) (DrawTimes :type Integer))
  (bind _size (Variables|Default|GetSize))
  (bind _currentt (Variables|Default|GetCurrentT))
  (bind (_location _rotation) (Math|Transform|BreakTransform _currentt))
  (bind _returnvalue (Math|Vector|GetForwardVector _rotation))
  (bind _returnvalue_2 (Math|Conversions|ToVector2D(Vector) _location))
  (bind _returnvalue_3 (Math|Rotator|MakeRotfromZX (Math|Vector|MakeVector 0.0 0.0 1.0) _returnvalue))
  (bind (_outscreenposition _outscreensize _outscreenrotation) (Class|WorldDrawingBoard|WorldtoCanvasBrush DrawingBoard _returnvalue_2 _size (.yaw _returnvalue_3)))
  (Canvas|DrawTexture :self CanvasDrawOn :RenderTexture (Variables|Pattern|GetRender%20Texture) :ScreenPosition _outscreenposition :ScreenSize _outscreensize :CoordinateSize (select (Variables|Pattern|GetMirrorFlip) "(X=-1.000000,Y=1.000000)" "(X=1.000000,Y=1.000000)") :BlendMode "BLEND_Additive" :Rotation _outscreenrotation :PivotPoint "(X=0.500000,Y=0.500000)"))

(fn UpdateDrawInfo
  (return true))