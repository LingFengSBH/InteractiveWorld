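; Brush component that stamps a depth capture of its owning actor onto a drawing board canvas.
; On BeginPlay it finds or spawns a single BP_SharedSceneCapture to borrow from.
; When draw info updates, that capture renders only the owner into TextureTarget, orthographically from 100 units below the trace point.
; DrawonRT feeds the texture to an M_DrawCapture material and draws it at the brush's canvas position and size.
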(event EventBeginPlay
  (|CallParentFunction)
  (bind _returnvalue (Actor|GetActorOfClass "/InteractiveWorld/Blueprints/Brushes/Master/BP_SharedSceneCapture.BP_SharedSceneCapture_C"))
  (Utilities|IsValid _returnvalue
    (:Is%20Valid
      (Variables|Default|SetSharedCapture _returnvalue))
    (:Is%20Not%20Valid
      (bind _returnvalue_2 (Game|SpawnActorfromClass "/InteractiveWorld/Blueprints/Brushes/Master/BP_SharedSceneCapture.BP_SharedSceneCapture_C" (Math|Transform|MakeTransform "0, 0, 0" "0, 0, 0" "1.000000,1.000000,1.000000") "Undefined" 0 0))
      (Variables|Default|SetSharedCapture _returnvalue_2))))

(event EventDrawonRT
  (params (DrawingBoard :type World%20Drawing%20Board%20Object%20Reference) (CanvasDrawOn :type Canvas%20Object%20Reference) (CanvasSize :type Vector%202D%20Structure) (InterpolateRate :type Float%20%28single-precision%29) (DrawTimes :type Integer))
  (bind _size (Variables|Default|GetSize))
  (bind _currentt (Variables|Default|GetCurrentT))
  (bind _returnvalue (Math|Conversions|ToVector2D(Vector) (.location _currentt)))
  (bind (_outscreenposition _outscreensize _outscreenrotation) (Class|WorldDrawingBoard|WorldtoCanvasBrush DrawingBoard _returnvalue _size 0.0))
  (bind _returnvalue_2 (Rendering|Material|CreateDynamicMaterialInstance "/InteractiveWorld/Materials/BrushMaterials/M_DrawCapture.M_DrawCapture" "None" "None" :!class /Script/Engine.KismetMaterialLibrary))
  (Rendering|Material|SetTextureParameterValue _returnvalue_2 "CaptureDepth" (Variables|CaptureSettings|GetTexture%20Target))
  (Rendering|Material|SetScalarParameterValue _returnvalue_2 "CameraOffset" -1e+02 :!class /Script/Engine.MaterialInstanceDynamic)
  (Canvas|DrawMaterial :self CanvasDrawOn :RenderMaterial _returnvalue_2 :ScreenPosition _outscreenposition :ScreenSize _outscreensize :CoordinateSize "(X=-1.000000,Y=1.000000)" :Rotation _outscreenrotation :PivotPoint "(X=0.500000,Y=0.500000)"))

(fn UpdateDrawInfo
  (bind _returnvalue (|CallParentFunction))
  (if _returnvalue
    (Default|BorrowSceneCapture (Variables|Default|GetSharedCapture) (Variables|CaptureSettings|GetTexture%20Target) (- (Variables|Default|GetTracePoint) "0,0,100.000000") (.x (Variables|Default|GetSize)) (Utilities|Array|MakeArray (Components|GetOwner)))
    (return true)
    (else
      (return false))))